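; GoalBP is a goal actor where a Sedan carrying the flag scores for its player.
; On Box overlap, the server toggles IsActive and increments the MyPlayerState score only when the goal turns inactive.
; SetMaterials then runs outside the authority check, swapping the goal's on/off material and firing the flag-captured dispatcher on the BP_GateManager found at BeginPlay.
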(event OnComponentBeginOverlap(Box)
  (params (OverlappedComponent :type Primitive%20Component%20Object%20Reference) (OtherActor :type Actor%20Object%20Reference) (OtherComp :type Primitive%20Component%20Object%20Reference) (OtherBodyIndex :type Integer) (bFromSweep :type Boolean) (SweepResult :type Hit%20Result%20Structure%20%28by%20ref%29))
  (bind _assedan (Utilities|Casting|CastToSedan OtherActor))
  (if (Variables|/Game/Blueprints/Sedan.Sedan_C|GethasFlag _assedan)
    (Utilities|FlowControl|Sequence
      (:then_0
        (Networking|SwitchHasAuthority
          (:Authority
            (bind _output_get (Variables|Default|SetisActive (not (Variables|Default|GetisActive))))
            (if (not _output_get)
              (bind _asmy_player_state (Utilities|Casting|CastToMyPlayerState (Variables|/Script/Engine.Pawn|GetPlayerState _assedan)))
              (Default|IncrementScore _asmy_player_state)))))
      (:then_1
        (CallFunction|SetMaterials (Variables|/Script/Engine.Pawn|GetPlayerState _assedan))))))

(event Custom|SetMaterials
  (params (PlayerState :type Player%20State%20Object%20Reference))
  (bind _goal (Variables|Default|GetGoal))
  (Utilities|Casting|CastToMyPlayerState PlayerState)
  (if (Variables|Default|GetisActive)
    (Rendering|Material|SetMaterial _goal 0 "/Game/Materials/Goal_Effect.Goal_Effect")
    (else
      (Rendering|Material|SetMaterial _goal 0 "/Game/Materials/Goal_Effect_Off.Goal_Effect_Off")))
  (Default|CallFlagCapturedEventDispatcher (Variables|Default|GetGateManager)))

(event EventBeginPlay
  (bind _outactors (Actor|GetAllActorsOfClass "/Game/Blueprints/BP_GateManager.BP_GateManager_C"))
  (if (> (Utilities|Array|Length _outactors) 0)
    (Variables|Default|SetGateManager (Utilities|Array|Get(acopy) _outactors))
    (else
      (Development|PrintString "UI_Minimap.Construct: BP_GateManager not found!" true true "(R=0.000000,G=0.660000,B=1.000000,A=1.000000)" 15.0))))

(event Collision|EventActorBeginOverlap
  (params (OtherActor :type Actor%20Object%20Reference)))

(event EventTick
  (params (DeltaSeconds :type Float%20%28single-precision%29)))

(fn ConstructionScript)